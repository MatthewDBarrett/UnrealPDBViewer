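; BP_QRCode is an actor, presumably displaying a QR code, that positions itself to face the SpaceMouseCamera when play begins.
; On BeginPlay it moves to a fixed distance from the world origin along a yaw-derived direction, using ring-spacing math hardcoded to a single slot.
; It then rotates once toward the camera's location with a look-at rotation, with no ongoing tracking.
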(event `self.ReceiveBeginPlay`
  (bind _returnvalue (`GameplayStatics.GetActorOfClass` "/DA_Assets/Camera/SpaceMouseCamera.SpaceMouseCamera_C"))
  (`self.K2_SetActorLocation` (+ (+ (* (`KismetMathLibrary.GetForwardVector` (`KismetMathLibrary.MakeRotator` 0.0 0.0 (`KismetMathLibrary.Conv_IntToDouble` (+ (* 0 (`KismetMathLibrary.FTrunc` (`KismetMathLibrary.Conv_IntToDouble` (/ 360 1)))) (`KismetMathLibrary.FTrunc` 180.0))))) 500.0) (0.0 0.0 0.0)) (0.0 0.0 0.0)))
  (`self.K2_SetActorRotation` (`KismetMathLibrary.FindLookAtRotation` (`self.K2_GetActorLocation`) (`self.K2_GetActorLocation` _returnvalue))))

(fn `UserConstructionScript`)