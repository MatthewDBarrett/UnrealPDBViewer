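; BP_Gallery spawns ButtonManager actors evenly around a circle at BeginPlay, marking each as a gallery item with its position and index.
; Positions come from yaw-stepped forward vectors scaled by Radius around CentreOfCircle, shifted by RotationOffset.
; A Quantity of six is special-cased to leave two slots empty.
; Each spawn also draws a debug circle raised by Height; a debug arrow is left unconnected.
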(event `self.ReceiveBeginPlay`
  (bind _quantity (`self.Quantity`))
  (for _index (range 1 (+ _quantity 1))
    (if (== (`self.Quantity`) 6)
      (if (and (and (!= _index 0) (!= _index 4)) (!= _index 5))
        (bind _returnvalue (+ (* (`KismetMathLibrary.GetForwardVector` (`KismetMathLibrary.MakeRotator` 0.0 0.0 (`KismetMathLibrary.Conv_IntToDouble` (+ (* _index (`KismetMathLibrary.FTrunc` (`KismetMathLibrary.Conv_IntToDouble` (/ 360 _quantity)))) (`KismetMathLibrary.FTrunc` (`self.Rotation Offset`)))))) (`self.Radius`)) (`self.Centre Of Circle`)))
        (bind _returnvalue_2 (`|SpawnActorFromClass` "/Game/ButtonManager.ButtonManager_C" (`KismetMathLibrary.MakeTransform` _returnvalue) "Undefined" "OverrideRootScale" null null :!label _label))
        (set `/Game/ButtonManager.Position` _returnvalue _returnvalue_2)
        (set `/Game/ButtonManager.isGallery` true _returnvalue_2)
        (set `/Game/ButtonManager.BM_Index` _index _returnvalue_2)
        (`KismetSystemLibrary.DrawDebugCircle` (+ (`self.Centre Of Circle`) (`KismetMathLibrary.MakeVector` 0.0 0.0 (`self.Height`))) (`self.Radius`) 100 (struct :`R` 1.0 :`G` 1.0 :`B` 1.0 :`A` 1.0) 50.0 20.0 (1.0 0.0 0.0) (0.0 1.0 0.0)))
      (else
        (goto _label)))))

(fn `UserConstructionScript`)